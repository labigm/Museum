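; BP_Frame is a museum picture frame that displays an artwork with its details and an optional audio description.
; The construction script sets the frame mesh and rotation, then applies a dynamic material with the picture texture and rotation to the "Picture" slot.
; Overlapping actors that implement BPI_MuseumCharacter receive title, artist, date, credit and description text while a 2D sound plays.
; Ending the overlap hides the text and stops the sound.
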(event EventBeginPlay)

(event Collision|EventActorBeginOverlap
  (params (OtherActor :type Actor%20Object%20Reference))
  (bind _sounddescription (Variables|Information|GetSoundDescription))
  (if (Utilities|DoesObjectImplementInterface OtherActor "/Game/Museum/Blueprints/BPI_MuseumCharacter.BPI_MuseumCharacter_C")
    (Class|BPIMuseumCharacter|DrawText(Message) OtherActor (Variables|Information|GetTitle) (Variables|Information|GetArtist) (Variables|Information|GetDate) (Variables|Information|GetCredit) (Variables|Information|GetDescription))
    (Utilities|IsValid _sounddescription
      (:Is%20Valid
        (bind _returnvalue (Audio|SpawnSound2D _sounddescription 1.0 1.0 0.0 0))
        (Variables|Default|SetSound _returnvalue)))))

(event Collision|EventActorEndOverlap
  (params (OtherActor :type Actor%20Object%20Reference))
  (bind _sound (Variables|Default|GetSound))
  (if (Utilities|DoesObjectImplementInterface OtherActor "/Game/Museum/Blueprints/BPI_MuseumCharacter.BPI_MuseumCharacter_C")
    (Class|BPIMuseumCharacter|HideText(Message) OtherActor)
    (Utilities|IsValid _sound
      (:Is%20Valid
        (Audio|Components|Audio|Stop _sound)))))

(fn ConstructionScript
  (Components|StaticMesh|SetStaticMesh (Variables|Default|GetStaticMesh) (Variables|Display|GetFrame))
  (bind _returnvalue (Rendering|Material|CreateDynamicMaterialInstance "/Game/Museum/Materials/M_Texture.M_Texture" "None" "None" :!class /Script/Engine.KismetMaterialLibrary))
  (Rendering|Material|SetTextureParameterValue _returnvalue "BaseColor" (Variables|Display|GetTexture))
  (Rendering|Material|SetScalarParameterValue _returnvalue "RotationAngle" (Variables|Display|GetPictureRotation) :!class /Script/Engine.MaterialInstanceDynamic)
  (Rendering|Material|SetMaterial (Variables|Default|GetStaticMesh) (Rendering|Material|GetMaterialIndex (Variables|Display|GetFrame) "Picture") _returnvalue)
  (Transformation|SetRelativeRotation (Variables|Default|GetStaticMesh) (Math|Rotator|MakeRotator 0.0 (Variables|Display|GetFrameRotation) -9e+01) false false))