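; Arch-viz controller that gives a placed actor interactive transform, visibility or color changes, selected by enum.
; At BeginPlay it inserts itself between that actor and its parent, caching transform and light or dynamic-material color.
; A press or awaited BPi_ArchViz call triggers the delayed action and notifies all interface implementers, enabling chains like switch to lights.
; Transforms snap or animate by timeline with linear or ping-pong loops; colors cycle through an enum.
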(event Custom|UserPressed
  ;[1 1 1] Will be called if the user actively selected this Blueprint. If EActivation was set to "Press", proceed
  (if (Utilities|Enum|Equal(Enum) (Variables|Settings|GetEActivation) "NewEnumerator2")
    (Utilities|FlowControl|Delay (Variables|AnimationSettings|GetDelayBeforeStart))
    (CallFunction|DetermineAction)))

(event Custom|Animate%20From%20End
  (bind _animating (Variables|AnimationSettings|GetAnimating))
  (bind _start_transform (Variables|Reference|GetStart%20Transform))
  (bind _end_transform (Variables|Action|GetEnd%20Transform))
  ;[1 1 1] Animation is prevented if the animation is playing
  (if (not _animating)
    (|SetBy-RefVar _animating true)
    ;[1 1 1] A minimal Timline with one changing value named Alpha. It will animate from 0 to 1 in 1 second linearly. We can use this value for many purposes.
    (bind (_direction _alpha) (Timeline|Animate_TL ReverseFromEnd)
      (:Update
        ;[1 1 1] Simple lerp from the start transform to the added "End Transform" designated by the user. Notice this is animating in Relative space.
        (Transformation|SetActorRelativeTransform (Math|Transform|Lerp(Transform) (Variables|Reference|GetStart%20Transform) (Math|Transform|MakeTransform (+ (.location _start_transform) (.location _end_transform)) (Math|Rotator|CombineRotators (.rotation _start_transform) (.rotation _end_transform)) (.scale _start_transform)) _alpha) false false))
      (:Finished
        ;[1 1 1] When animation finished, send the Direction Enumeration to decide what to do next based on which direction just played
        (CallFunction|AnimationHasFinished _direction)))))

(event Custom|Animate%20From%20Start
  (bind _animating (Variables|AnimationSettings|GetAnimating))
  (bind _start_transform (Variables|Reference|GetStart%20Transform))
  (bind _end_transform (Variables|Action|GetEnd%20Transform))
  ;[1 1 1] Animation is prevented if the animation is playing
  (if (not _animating)
    (|SetBy-RefVar _animating true)
    ;[1 1 1] A minimal Timline with one changing value named Alpha. It will animate from 0 to 1 in 1 second linearly. We can use this value for many purposes.
    (bind (_direction _alpha) (Timeline|Animate_TL PlayFromStart)
      (:Update
        ;[1 1 1] Simple lerp from the start transform to the added "End Transform" designated by the user. Notice this is animating in Relative space.
        (Transformation|SetActorRelativeTransform (Math|Transform|Lerp(Transform) (Variables|Reference|GetStart%20Transform) (Math|Transform|MakeTransform (+ (.location _start_transform) (.location _end_transform)) (Math|Rotator|CombineRotators (.rotation _start_transform) (.rotation _end_transform)) (.scale _start_transform)) _alpha) false false))
      (:Finished
        ;[1 1 1] When animation finished, send the Direction Enumeration to decide what to do next based on which direction just played
        (CallFunction|AnimationHasFinished _direction)))))

(event Custom|DetermineAction
  (bind _reverseanimation (Variables|AnimationSettings|GetReverseAnimation))
  ;[1 1 1] If the User has initiated action successfully, call the interface that this is launched. Perhaps another Blueprint is waiting on this one to be called. (Ex. a lightswitch won't do anything to itself, but it will call to the listening lights to activate/deactive)
  (CallFunction|CallInterfacetoInitiateAction)
  (switch Utilities|FlowControl|Switch|SwitchonEAction (Variables|Settings|GetEAction)
    (:NewEnumerator1
      ;[1 1 1] Determine the type of Transform change
      (if (Variables|AnimationSettings|GetShouldAnimate)
        (if _reverseanimation
          (|SetBy-RefVar _reverseanimation false)
          (CallFunction|AnimatefromEnd)
          (else
            (CallFunction|AnimatefromStart)))
        (else
          (CallFunction|FlipFlopTransform))))
    (:NewEnumerator2
      ;[1 1 1] Check if Actor is visible or not and toggle to the NOT value.
      (Variables|AnimationSettings|SetToggleVisibility (not (Variables|AnimationSettings|GetToggleVisibility)))
      (Rendering|SetVisibility (Variables|/Script/Engine.Actor|GetRootComponent (Variables|Reference|GetOriginalParent)) (Variables|AnimationSettings|GetToggleVisibility) true))
    (:NewEnumerator4
      ;[1 1 1] Using the current value of EColor, select a new color
      (bind _newcolor (CallFunction|CycleLinearColor false))
      ;[1 1 1] If light, set the new color to the light
      (bind _aslight (Utilities|Casting|CastToLight (Variables|Reference|GetOriginalParent))
        (:then
          (Rendering|Components|Light|SetLightColor (Variables|/Script/Engine.Light|GetLightComponent _aslight) _newcolor true))
        (:CastFailed
          ;[1 1 1] If static mesh has a valid material Vector parameter, set the value to the new color
          (Utilities|IsValid (Variables|ColorChange|GetMaterialToChange)
            (:Is%20Valid
              (Rendering|Material|SetVectorParameterValue (Variables|ColorChange|GetMaterialToChange) (Variables|ColorChange|GetParameterName) _newcolor :!class /Script/Engine.MaterialInstanceDynamic))))))))

(event Custom|FlipFlop%20Transform
  (bind _end_transform (Variables|Action|GetEnd%20Transform))
  (bind _start_transform (Variables|Reference|GetStart%20Transform))
  ;[1 1 1] If the user does not set the variable "Should Animate" to true, the motion of the Actor will simply snap to the new transfrom.
  (bind _isa (Utilities|FlowControl|FlipFlop)
    (:A
      _)
    (:B
      _))
  (Transformation|SetActorRelativeTransform (Math|Transform|SelectTransform (Math|Transform|MakeTransform (+ (.location _start_transform) (.location _end_transform)) (Math|Rotator|CombineRotators (.rotation _start_transform) (.rotation _end_transform)) (.scale _start_transform)) (Variables|Reference|GetStart%20Transform) _isa) false false))

(event Custom|Animation%20has%20finished
  (params (InputPin :type ETimelineDirection%20Enum :default "Forward"))
  ;[1 1 1] Animation has finished. Set "Animating" to false so it can be called again.
  (Variables|AnimationSettings|SetAnimating false)
  ;[1 1 1] Check if the animation loop has finished.
  (if (== (Variables|AnimationSettings|GetAnimationLoopCount) 0)
    ;[1 1 1] Restore the original Animation Loop Count
    (bind _output_get (Variables|AnimationSettings|SetAnimationLoopCount (Variables|Animation|GetAnimationLoopCount_Start)))
    ;[1 1 1] If the animation loop has finished and the original Animation Loop was set to 0 (as in, only play once) and "EAnimationSettings" was set to PingPong, this means that the user wanted to be able to Undo the effect of the animation. An example would be a door. We want it to animate open once. But if called again, we would want it to animate closed aas well, without looping.
    (if (== _output_get 0)
      (switch Utilities|FlowControl|Switch|SwitchonEAnimationSettings (Variables|Animation|GetEAnimationSettings)
        (:NewEnumerator1
          ;;[1 1 1] This second bool "AnimationShouldPlayReversed" has been added so that when an animation should be reset and start again from the beginning and not at the end, it can be reset using the "NOT" node
          (Variables|AnimationSettings|SetReverseAnimation (not (Variables|AnimationSettings|GetAnimationShouldPlayReversed)))
          (Variables|AnimationSettings|SetAnimationShouldPlayReversed (not (Variables|AnimationSettings|GetAnimationShouldPlayReversed))))))
    (else
      ;[1 1 1] Loop the animation until "AnimationLoopCount" equals 0. "AnimationLoopCount" will not go down unless a finished Forward animation completed. Backwards animation does not count against this count.
      (switch Utilities|FlowControl|Switch|SwitchonETimelineDirection InputPin
        (:Forward
          ;;[1 1 1] Linear animation will alaways play a forward animation while a PingPong animation will go back and forth.
          (switch Utilities|FlowControl|Switch|SwitchonEAnimationSettings (Variables|Animation|GetEAnimationSettings)
            (:NewEnumerator0
              (CallFunction|AnimatefromStart))
            (:NewEnumerator1
              (CallFunction|AnimatefromEnd)))
          (if (not (== (Variables|AnimationSettings|GetAnimationLoopCount) -1))
            (Math|Integer|DecrementInt (Variables|AnimationSettings|GetAnimationLoopCount))))
        (:Backward
          (CallFunction|AnimatefromStart))))))

(event EventBeginPlay
  (bind _originalparent (Variables|Reference|GetOriginalParent))
  ;[1 1 1] Allow a small amount of time to make sure the Blueprints are spawned and ready.
  (Utilities|FlowControl|Delay 0.2)
  ;[1 1 1] For us to attach the original object, it must be set to movable
  (Utilities|IsValid _originalparent
    (:Is%20Valid
      (Transformation|SetMobility (Variables|/Script/Engine.Actor|GetRootComponent _originalparent) "Movable")
      ;[1 1 1] We have two attachments as we want to keep the original hierachy. First, parent this new Blueprint to the original's parent. Then parent the original Blueprint to this one.
      (Transformation|AttachActorToActor self (Actor|GetAttachParentActor (Variables|Reference|GetOriginalParent)) "None" "KeepWorld" "KeepWorld" "KeepWorld" true)
      (Transformation|AttachActorToActor (Variables|Reference|GetOriginalParent) self "None" "KeepWorld" "KeepWorld" "KeepWorld" true)
      ;[1 1 1] Cache reference data for later usage
      (Variables|Reference|SetStart%20Transform (Transformation|GetRelativeTransform (Variables|Default|GetDefaultSceneRoot self)))
      (Variables|Animation|SetAnimationLoopCount_Start (Variables|AnimationSettings|GetAnimationLoopCount))
      (Variables|AnimationSettings|SetToggleVisibility (Variables|/Script/Engine.SceneComponent|GetbVisible (Variables|/Script/Engine.Actor|GetRootComponent (Variables|Reference|GetOriginalParent))))
      ;;[1 1 1] Provides a value to the original color in EColor
      (CallFunction|GetOriginalColor)
      ;[1 1 1] One time value set for the animation play rate. The high the number, the quicker it plays.
      (Components|Timeline|SetPlayRate (Variables|Default|GetAnimate_TL) (Variables|AnimationSettings|GetAnimationPlayRate)))))

(event EventUserInitiatedAction
  (params (CallMadeBy :type Actor%20Object%20Reference))
  ;[1 1 1] Another Blueprint has called this function in our Interface, if we are waiting for that call from that specific Actor, proceed.
  (if (and (Utilities|Enum|Equal(Enum) (Variables|Settings|GetEActivation) "NewEnumerator3") (== CallMadeBy (Variables|Action|GetActorToWaitFor)))
    (Utilities|FlowControl|Delay (Variables|AnimationSettings|GetDelayBeforeStart))
    (CallFunction|DetermineAction)))

(fn ConstructionScript)

(fn CallInterfacetoInitiateAction
  ;[1 1 1] Call the function "User Initiated Action" in all Blueprints that implement our BPi_ArchViz
  (bind _outactors (Actor|GetAllActorswithInterface "/Game/UsingEnums/ArchVizInt/Blueprints/Interface/BPi_ArchViz.BPi_ArchViz_C"))
  (for _array_element _outactors
    (Class|BPiArchViz|UserInitiatedAction(Message) _array_element (Variables|Reference|GetOriginalParent))))

(fn CycleLinearColor
  (params (ManualSelection :type Boolean))
  (if ManualSelection
    ;[1 1 1] Manual selection of which color to change to based on which color it was.
    (Variables|ColorChange|SetEColor (Utilities|Select :Index (Variables|ColorChange|GetEColor) :NewEnumerator7 "NewEnumerator5" :NewEnumerator0 "NewEnumerator3" :NewEnumerator1 "NewEnumerator4" :NewEnumerator2 "NewEnumerator1" :NewEnumerator3 "NewEnumerator2" :NewEnumerator4 "NewEnumerator6" :NewEnumerator5 "NewEnumerator0" :NewEnumerator6 "NewEnumerator7"))
    (else
      ;[1 1 1] If the value of EColor is its max value, it will be reset to the value of '0' which equals the original color
      (if (>= (Math|Conversions|ToInteger(Byte) (Variables|ColorChange|GetEColor)) (- (|GetNumEnumEntries) 1))
        (Variables|ColorChange|SetEColor (Utilities|Enum|ByteToEnumEColor))
        (else
          (Variables|ColorChange|SetEColor (Utilities|Enum|ByteToEnumEColor (+ (Variables|ColorChange|GetEColor) 1)))))))
  ;[1 1 1] Useing the Select node together with an Enum allows us to set different values bases on the value of the enum itself.
  (return (Utilities|Select :Index (Variables|ColorChange|GetEColor) :NewEnumerator7 (Variables|ColorChange|GetOriginalColor) :NewEnumerator0 "(R=1.000000,G=0.100000,B=0.100000,A=1.000000)" :NewEnumerator1 "(R=1.000000,G=0.451430,B=0.100000,A=1.000000)" :NewEnumerator2 "(R=1.000000,G=0.845113,B=0.100000,A=1.000000)" :NewEnumerator3 "(R=0.411164,G=1.000000,B=0.100000,A=1.000000)" :NewEnumerator4 "(R=0.100000,G=1.000000,B=0.975294,A=1.000000)" :NewEnumerator5 "(R=0.100000,G=0.212562,B=1.000000,A=1.000000)" :NewEnumerator6 "(R=0.363406,G=0.100000,B=1.000000,A=1.000000)")))

(fn GetOriginalColor
  (bind _originalparent (Variables|Reference|GetOriginalParent))
  ;[1 1 1] If the Actor is a light, we need to cast specifically to the parent of the actor. If it is not a light, the cast will fail and we assume it is a StaticMeshActor
  (bind _aslight (Utilities|Casting|CastToLight _originalparent)
    (:then
      (Variables|ColorChange|SetOriginalColor (Math|Conversions|ToLinearColor(Color) (Variables|/Script/Engine.LightComponentBase|GetLightColor (Variables|/Script/Engine.Light|GetLightComponent _aslight)))))
    (:CastFailed
      ;[1 1 1] Casts to StaticMeshActor and creates a DynamicMaterial Instance. This will allow us to alter parameters setup inside the material.
      (bind _asstatic_mesh_actor (Utilities|Casting|CastToStaticMeshActor _originalparent))
      (bind _returnvalue (Rendering|Material|CreateDynamicMaterialInstance (Variables|/Script/Engine.StaticMeshActor|GetStaticMeshComponent _asstatic_mesh_actor) (Variables|ColorChange|GetMaterialIDsToChange) 0 "None" :!class /Script/Engine.PrimitiveComponent))
      (bind _output_get (Variables|ColorChange|SetMaterialToChange _returnvalue))
      ;;[1 1 1] Cache the original color inside of the material
      (bind _returnvalue_2 (Rendering|Material|GetVectorParameterValue _output_get (Variables|ColorChange|GetParameterName) :!class /Script/Engine.MaterialInstanceDynamic))
      (Variables|ColorChange|SetOriginalColor _returnvalue_2))))