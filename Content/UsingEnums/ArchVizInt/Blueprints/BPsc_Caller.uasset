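; BPsc_Caller is a scene component that exposes interaction and animation settings and hands the work to a separate controller Blueprint.
; On BeginPlay it spawns a BP_Controller at its world transform and stores the reference.
; It then copies its action, activation, animation, material, timing, end transform and wait-for actor settings onto that controller, along with its owner as OriginalParent.
; The mechanics themselves live in BP_Controller.
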(event EventBeginPlay
  ;[1 1 1] Spawn the Blueprint that handles the actual mechanics
  (bind _returnvalue (Game|SpawnActorfromClass "/Game/UsingEnums/ArchVizInt/Blueprints/BP_Controller.BP_Controller_C" (Transformation|GetWorldTransform self) "Undefined" 0 0))
  (Variables|Spawned|SetSpawnedController _returnvalue)
  ;[1 1 1] Pass on all the values to user has chosed to the new Blueprint to prepare it for use
  (Variables|/Game/UsingEnums/ArchVizInt/Blueprints/BP_Controller.BP_Controller_C|SetEAction (Variables|Spawned|GetSpawnedController) (Variables|Settings|GetEAction))
  (Variables|/Game/UsingEnums/ArchVizInt/Blueprints/BP_Controller.BP_Controller_C|SetEActivation (Variables|Spawned|GetSpawnedController) (Variables|Settings|GetEActivation))
  (Variables|/Game/UsingEnums/ArchVizInt/Blueprints/BP_Controller.BP_Controller_C|SetEAnimationSettings (Variables|Spawned|GetSpawnedController) (Variables|Animation|GetEAnimationSettings))
  (Variables|/Game/UsingEnums/ArchVizInt/Blueprints/BP_Controller.BP_Controller_C|SetShouldAnimate (Variables|Spawned|GetSpawnedController) (Variables|Animation|GetShouldAnimate))
  (Variables|/Game/UsingEnums/ArchVizInt/Blueprints/BP_Controller.BP_Controller_C|SetMaterialIDsToChange (Variables|Spawned|GetSpawnedController) (Variables|MaterialChange|GetMaterialIDToChange))
  (Variables|/Game/UsingEnums/ArchVizInt/Blueprints/BP_Controller.BP_Controller_C|SetParameterName (Variables|Spawned|GetSpawnedController) (Variables|MaterialChange|GetParameterName))
  (Variables|/Game/UsingEnums/ArchVizInt/Blueprints/BP_Controller.BP_Controller_C|SetDelayBeforeStart (Variables|Spawned|GetSpawnedController) (Variables|Animation|GetDelayBeforeStart))
  (Variables|/Game/UsingEnums/ArchVizInt/Blueprints/BP_Controller.BP_Controller_C|SetAnimationPlayRate (Variables|Spawned|GetSpawnedController) (Variables|Animation|GetAnimationPlayRate))
  (Variables|/Game/UsingEnums/ArchVizInt/Blueprints/BP_Controller.BP_Controller_C|SetAnimationLoopCount (Variables|Spawned|GetSpawnedController) (Variables|Animation|GetAnimationLoopCount%20%28-1%20for%20Infinite%29))
  (Variables|/Game/UsingEnums/ArchVizInt/Blueprints/BP_Controller.BP_Controller_C|SetEnd%20Transform (Variables|Spawned|GetSpawnedController) (Variables|Action|GetEndTransform%20%28AdditiveNoScale%29))
  (Variables|/Game/UsingEnums/ArchVizInt/Blueprints/BP_Controller.BP_Controller_C|SetActorToWaitFor (Variables|Spawned|GetSpawnedController) (Variables|Action|GetActorToWaitFor))
  (Variables|/Game/UsingEnums/ArchVizInt/Blueprints/BP_Controller.BP_Controller_C|SetOriginalParent (Variables|Spawned|GetSpawnedController) (Components|GetOwner self)))